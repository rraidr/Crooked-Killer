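; BloodBag_BP is a health pickup that restores the ThirdPersonCharacter's Health.
; On box overlap it adds BloodBagValue, clamped between zero and one, then destroys itself, unless health is already full.
; Tick spins the root around yaw, while BeginPlay runs a timed lifetime that blinks the bag and aura fire through repeated visibility toggles before destroying the actor.
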(event OnComponentBeginOverlap(Box)
  (params (OverlappedComponent :type Primitive%20Component%20Object%20Reference) (OtherActor :type Actor%20Object%20Reference) (OtherComp :type Primitive%20Component%20Object%20Reference) (OtherBodyIndex :type Integer) (bFromSweep :type Boolean) (SweepResult :type Hit%20Result%20Structure%20%28by%20ref%29))
  (bind _asthird_person_character (Utilities|Casting|CastToThirdPersonCharacter OtherActor))
  (if (not (== (Variables|/Game/ThirdPersonBP/Blueprints/ThirdPersonCharacter.ThirdPersonCharacter_C|GetHealth _asthird_person_character) 1.0))
    (Variables|/Game/ThirdPersonBP/Blueprints/ThirdPersonCharacter.ThirdPersonCharacter_C|SetHealth _asthird_person_character (Math|Float|Clamp(Float) (+ (Variables|Default|GetBloodBagValue) (Variables|/Game/ThirdPersonBP/Blueprints/ThirdPersonCharacter.ThirdPersonCharacter_C|GetHealth _asthird_person_character))))
    (Actor|DestroyActor)))

(event EventBeginPlay
  (Utilities|FlowControl|Delay 1e+01)
  (Rendering|ToggleVisibility (Variables|Default|GetBloodBag) false)
  (Utilities|FlowControl|Delay 0.5)
  (Rendering|ToggleVisibility (Variables|Default|GetBloodBag) false)
  (Utilities|FlowControl|Delay 0.5)
  (Rendering|ToggleVisibility (Variables|Default|GetBloodBag) false)
  (Utilities|FlowControl|Delay 0.5)
  (Rendering|ToggleVisibility (Variables|Default|GetBloodBag) false)
  (Utilities|FlowControl|Delay 0.5)
  (Rendering|ToggleVisibility (Variables|Default|GetBloodBag) false)
  (Utilities|FlowControl|Delay 0.5)
  (Rendering|ToggleVisibility (Variables|Default|GetBloodBag) false)
  (Utilities|FlowControl|Delay 0.5)
  (Actor|DestroyActor))

(event EventTick
  (params (DeltaSeconds :type Float%20%28single-precision%29))
  (bind _defaultsceneroot (Variables|Default|GetDefaultSceneRoot))
  (bind _returnvalue (Transformation|GetWorldRotation _defaultsceneroot))
  (bind (_roll _pitch _yaw) (Math|Rotator|BreakRotator _returnvalue))
  (bind _result (Math|Float|IncrementFloat DeltaSeconds)
    (:%20%20
      (Transformation|SetWorldRotation _defaultsceneroot (Math|Rotator|MakeRotator _roll _pitch (+ _yaw (* _result 1.0))) false false))))

(fn ConstructionScript)